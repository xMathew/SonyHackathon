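; GameHUD is a HUD Blueprint that draws a center crosshair and an indicator of the player's current paint color.
; Each DrawHUD call draws a small purple square from the screen's midpoint, then casts player character 0 to Player.
; It switches on that Player's PaintColor to draw a larger gray, white or red swatch near the bottom-right corner.
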(event EventDrawHUD
  (params (SizeX :type Integer) (SizeY :type Integer))
  (bind _returnvalue (- SizeX 100))
  (bind _returnvalue_2 (- SizeY 100))
  (bind _returnvalue_3 (Math|Conversions|ToFloat(Integer) _returnvalue))
  (bind _returnvalue_4 (Math|Conversions|ToFloat(Integer) _returnvalue_2))
  (HUD|DrawRect "(R=0.380000,G=0.250800,B=0.362435,A=1.000000)" (Math|Conversions|ToFloat(Integer) (/ SizeX 2)) (Math|Conversions|ToFloat(Integer) (/ SizeY 2)) 1e+01 1e+01)
  (bind _asplayer_c (Utilities|Casting|CastToPlayer (Game|GetPlayerCharacter 0)))
  (switch int (Variables|/Game/Blueprints/GameBlueprints/Player.Player_C|GetPaintColor _asplayer_c)
    (:0
      (HUD|DrawRect (Math|Color|MakeColor 0.495 0.495 0.495) _returnvalue_3 _returnvalue_4 5e+01 5e+01))
    (:1
      (HUD|DrawRect (Math|Color|MakeColor 1.0 1.0 1.0) _returnvalue_3 _returnvalue_4 5e+01 5e+01))
    (:2
      (HUD|DrawRect (Math|Color|MakeColor 1.0 0.0 0.0) _returnvalue_3 _returnvalue_4 5e+01 5e+01))))

(fn ConstructionScript)